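; Looping-corridor start segment that spawns the next corridor piece as the player walks through it.
; On the player's first overlap with its Box, it locks and closes its child-actor door and destroys any valid previous corridor.
; It then spawns a loop-end corridor at NewCorridorPlacement with the loop count reset to zero.
; Counter-based logic for repeating start segments until LoopUntilSwitch is left disconnected.
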(event `self.ReceiveBeginPlay`
  (bind _asbp_lockable_door (cast `/Game/Blueprints/Interactables/BP_Lockable_Door` (`ChildActorComponent.ChildActor` (`self.BP_Lockable_Door`))))
  (set `self.lockable_door` _asbp_lockable_door)
  (`KismetSystemLibrary.PrintText` (`KismetTextLibrary.Conv_IntToText` (`self.Loop_Number`))))

(event `self.Box.OnComponentBeginOverlap`
  (params (OverlappedComponent :type "PrimitiveComponent Object Reference") (OtherActor :type "Actor Object Reference") (OtherComp :type "PrimitiveComponent Object Reference") (OtherBodyIndex :type Integer) (bFromSweep :type Boolean) (SweepResult :type "HitResult Structure (by ref)"))
  (bind _lockable_door (`self.lockable_door`))
  (bind _previouscorridor (`self.PreviousCorridor`))
  (if (and (== OtherActor (`Controller.K2_GetPawn` (`GameplayStatics.GetPlayerController` 0))) (not (`self.HasBeenThrough`)))
    (set `self.HasBeenThrough` true)
    (`/Game/Blueprints/Interactables/BP_Lockable_Door.LockDoor` _lockable_door)
    (`/Game/Blueprints/Interactables/BP_Door.CloseDoor` _lockable_door)
    (`|ExecutionSequence`
      (:`then_0`
        (`/Engine/EditorBlueprintResources/StandardMacros.IsValid` _previouscorridor
          (:`Is Valid`
            (`self.K2_DestroyActor` _previouscorridor))))
      (:`then_1`
        (bind _returnvalue (`|SpawnActorFromClass` "/Game/LabyinthCorridors/bp_loop_end_Test.bp_loop_end_Test_C" (`SceneComponent.K2_GetComponentToWorld` (`self.NewCorridorPlacement`)) "Undefined" "OverrideRootScale" null null))
        (set `self.PreviousCorridor` self)
        (set `/Game/LabyinthCorridors/bp_loop_end_Test.Loop_Number` 0 _returnvalue)
        (`KismetSystemLibrary.PrintText` "NEW LOOP STARTED")))))

(fn `UserConstructionScript`)