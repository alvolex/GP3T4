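; BP_Planet is a planet actor whose graph handles its explosion when destroyed.
; On its OnDestroy event it spawns a BP_BigExplosion at its location, with rotation derived from the DeathHit normal.
; It multiplies the effect's scale, spawn radius and particle speed range by the length of the planet's scale vector, then activates it, so the blast grows with planet size.
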(event `self.ReceiveOnDestroy`
  (bind _returnvalue (`KismetMathLibrary.VSize` (`self.GetActorScale3D`)))
  (bind _returnvalue_2 (`|SpawnActorFromClass` "/Game/VFX/BP_BigExplosion.BP_BigExplosion_C" (`KismetMathLibrary.MakeTransform` (`self.K2_GetActorLocation`) (`KismetMathLibrary.MakeRotator` (.pitch (`KismetMathLibrary.MakeRotFromZ` (`.Normal` (`GameplayStatics.BreakHitResult` (`self.DeathHit`))))) (.roll (`KismetMathLibrary.MakeRotFromZ` (`.Normal` (`GameplayStatics.BreakHitResult` (`self.DeathHit`))))) (+ (.yaw (`KismetMathLibrary.MakeRotFromZ` (`.Normal` (`GameplayStatics.BreakHitResult` (`self.DeathHit`))))) -90.0))) "Undefined" "OverrideRootScale" null null))
  (bind _explosioneffect (`/Game/VFX/BP_BigExplosion.ExplosionEffect` _returnvalue_2))
  (`FXSystemComponent.SetFloatParameter` _explosioneffect "Scale Factor" (* 3.0 _returnvalue))
  (`FXSystemComponent.SetFloatParameter` _explosioneffect "Spawn Radius" (* 120.0 _returnvalue))
  (`FXSystemComponent.SetFloatParameter` _explosioneffect "Min Speed" (* 100.0 _returnvalue))
  (`FXSystemComponent.SetFloatParameter` _explosioneffect "Max Speed" (* 3000.0 _returnvalue))
  (`ActorComponent.Activate` _explosioneffect false))

(fn `UserConstructionScript`)