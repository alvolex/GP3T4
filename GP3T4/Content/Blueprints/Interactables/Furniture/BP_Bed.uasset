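; Interactable bed that, once used, puts the player to sleep and runs the bedroom-to-space transition.
; A dreaming FMOD event leads into locking player input at the sleep position and fading to black via the HUD fade widget before BedroomToSpace runs.
; Afterwards it fades back in, switches the lights off and unlocks the player at the wake-up position.
; Older post-process blend and level-loading logic remains but never runs.
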(event `self.ReceiveBeginPlay`
  (bind _asgp3t4character (cast `GP3T4Character` (`GameplayStatics.GetPlayerCharacter` 0))
    (:`then`
      (set `self.Player` _asgp3t4character))
    (:`CastFailed`
      (`KismetSystemLibrary.PrintText` "Player not found in BP_Bed" true true (struct :`R` 0.973601 :`G` 0.305747 :`B` 1.0 :`A` 1.0) 5.0))))

(event `self.ReceiveInteractWithObject`
  (bind _sleepposition (`self.SleepPosition`))
  (bind _wakeupposition (`self.WakeUpPosition`))
  (bind _fade_in_duration (`self.Fade_IN_Duration`))
  (bind _fade_out_duration (`self.Fade_OUT_Duration`))
  ;[0.1558 0.06737 0.349] To Space
  (`/Engine/EditorBlueprintResources/StandardMacros.DoOnce` false
    (:`Completed`
      (`/Game/Blueprints/Macros/BP_FMODMacros.PlayFMODEvent` "/Game/FMOD/Events/Dreaming.Dreaming" (`SceneComponent.K2_GetComponentToWorld` (`self.SleepPosition`))
        (:`Finish`
          (`GP3T4Character.LockInputAtSleep` (`self.Player`) true (`SceneComponent.K2_GetComponentLocation` _sleepposition) (`SceneComponent.K2_GetComponentRotation` _sleepposition))
          (`self.FadeToBlack` _fade_in_duration)
          (`KismetSystemLibrary.Delay` _fade_in_duration)
          (`/Game/Blueprints/Macros/BP_LevelTransitionMacros.BedroomToSpace`
            (:`End`
              (`KismetSystemLibrary.Delay` (`self.Fade_HOLD_Duration`))
              (`self.FadeToNormal` _fade_out_duration)
              (`KismetSystemLibrary.Delay` _fade_out_duration)
              (`GP3T4Character.LockInputAtSleep` (`self.Player`) false (`SceneComponent.K2_GetComponentLocation` _wakeupposition) (`SceneComponent.K2_GetComponentRotation` _wakeupposition)))))))))

(event `InterpPP`
  ;[1 1 1] OLD stuff
)

(event `FinishedFade`
  ;[1 1 1] OLD stuff
)

(fn `FadeToBlack`
  (params (FadeInDuration :type "Float (double-precision)"))
  (bind _asbp_player_hud (cast `/Game/Blueprints/HUD/BP_PlayerHUD` (`PlayerController.GetHUD` (`GameplayStatics.GetPlayerController` 0))))
  (bind _fadewidget (`/Game/Blueprints/HUD/BP_PlayerHUD.FadeWidget` _asbp_player_hud))
  (`/Game/Dans_Hyperbolic_Anxiety_chamber/Fade.FadeToBlack` _fadewidget FadeInDuration "Forward")
  (`UserWidget.BindToAnimationFinished` _fadewidget (`/Game/Dans_Hyperbolic_Anxiety_chamber/Fade.FadeInBlackScreen` _fadewidget) (`|CreateDelegate` :!event `FinishedFade`)))

(fn `FadeToNormal`
  (params (FadeOutDuration :type "Float (double-precision)"))
  (bind _asbp_player_hud (cast `/Game/Blueprints/HUD/BP_PlayerHUD` (`PlayerController.GetHUD` (`GameplayStatics.GetPlayerController` 0))))
  (bind _fadewidget (`/Game/Blueprints/HUD/BP_PlayerHUD.FadeWidget` _asbp_player_hud))
  (`UserWidget.UnbindFromAnimationFinished` _fadewidget (`/Game/Dans_Hyperbolic_Anxiety_chamber/Fade.FadeInBlackScreen` _fadewidget) (`|CreateDelegate` :!event `FinishedFade`))
  (`/Game/Dans_Hyperbolic_Anxiety_chamber/Fade.FadeToBlack` _fadewidget FadeOutDuration "Reverse")
  (`/Game/Blueprints/Interactables/Furniture/BP_LightSwitch.SetLights` (`self.LightSwitch`) false))

(fn `UserConstructionScript`)