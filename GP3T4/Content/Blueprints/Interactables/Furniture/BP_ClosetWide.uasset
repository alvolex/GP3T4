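; Interactable wide closet that toggles open and closed, sliding its drawer and swinging both doors together.
; BeginPlay caches each part's starting transform and computes its open pose as a relative offset.
; Interaction, ignored while animating, plays the same FMOD wardrobe sound for either direction, then calls Open or Close from its Finish output.
; Separate timelines lerp the parts between poses, updating the open state when finished.
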(event `self.ReceiveBeginPlay`
  (bind _relativelocation (`SceneComponent.RelativeLocation` (`self.SM_closet_wide_drawer`)))
  (bind _relativerotation (`SceneComponent.RelativeRotation` (`self.SM_closet_wide_door_L`)))
  (bind _relativerotation_2 (`SceneComponent.RelativeRotation` (`self.SM_closet_wide_door_R`)))
  ;[0.3577 1 0.9102] Set values for animations
  (set `self.DrawerStart` _relativelocation)
  (set `self.DrawerEnd` (`KismetMathLibrary.MakeVector` (.x _relativelocation) (+ (.y _relativelocation) 40.0) (.z _relativelocation)))
  (set `self.DoorLStart` _relativerotation)
  (set `self.DoorLEnd` (`KismetMathLibrary.MakeRotator` (.roll _relativerotation) (.pitch _relativerotation) (- (.yaw _relativerotation) 90.0)))
  (set `self.DoorRStart` _relativerotation_2)
  (set `self.DoorREnd` (`KismetMathLibrary.MakeRotator` (.roll _relativerotation_2) (.pitch _relativerotation_2) (+ (.yaw _relativerotation_2) 90.0))))

(event `self.ReceiveInteractWithObject`
  (bind _returnvalue (`self.GetTransform`))
  (if (`self.IsAnimating`)
    _
    (elif (`self.IsOpen`)
      (`/Game/Blueprints/Macros/BP_FMODMacros.PlayFMODEvent` "/Game/FMOD/Events/Wardrobeopen.Wardrobeopen" _returnvalue
        (:`Finish`
          (`self.Close`)))
      (else
        (`/Game/Blueprints/Macros/BP_FMODMacros.PlayFMODEvent` "/Game/FMOD/Events/Wardrobeopen.Wardrobeopen" _returnvalue
          (:`Finish`
            (`self.Open`)))))))

(event `Open`
  ;[0.5724 1 0.6015] Open
  (set `self.IsAnimating` true)
  (bind (_direction _alpha) (`Timeline|OpenTimeLine` :!via `PlayFromStart`)
    (:`Update`
      (`SceneComponent.K2_SetRelativeLocation` (`self.SM_closet_wide_drawer`) (`KismetMathLibrary.VLerp` (`self.DrawerStart`) (`self.DrawerEnd`) _alpha) false false)
      (`SceneComponent.K2_SetRelativeRotation` (`self.SM_closet_wide_door_L`) (`KismetMathLibrary.RLerp` (`self.DoorLStart`) (`self.DoorLEnd`) _alpha true) false false)
      (`SceneComponent.K2_SetRelativeRotation` (`self.SM_closet_wide_door_R`) (`KismetMathLibrary.RLerp` (`self.DoorRStart`) (`self.DoorREnd`) _alpha true) false false))
    (:`Finished`
      (set `self.IsAnimating` false)
      (set `self.IsOpen` true))))

(event `Close`
  ;[1 0.6224 0.5925] Close
  (set `self.IsAnimating` true)
  (bind (_direction _alpha) (`Timeline|CloseTimeLine` :!via `PlayFromStart`)
    (:`Update`
      (`SceneComponent.K2_SetRelativeLocation` (`self.SM_closet_wide_drawer`) (`KismetMathLibrary.VLerp` (`self.DrawerEnd`) (`self.DrawerStart`) _alpha) false false)
      (`SceneComponent.K2_SetRelativeRotation` (`self.SM_closet_wide_door_L`) (`KismetMathLibrary.RLerp` (`self.DoorLEnd`) (`self.DoorLStart`) _alpha true) false false)
      (`SceneComponent.K2_SetRelativeRotation` (`self.SM_closet_wide_door_R`) (`KismetMathLibrary.RLerp` (`self.DoorREnd`) (`self.DoorRStart`) _alpha true) false false))
    (:`Finished`
      (set `self.IsAnimating` false)
      (set `self.IsOpen` false))))

(fn `UserConstructionScript`)