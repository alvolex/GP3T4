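; Lockable door interactable that gates its parent class's interaction behind a lock state.
; InteractWithObject passes through to the parent implementation only while IsLocked is false, and otherwise does nothing.
; LockDoor and UnlockDoor set the IsLocked flag, with no key check or feedback in this Blueprint.
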(event `self.ReceiveInteractWithObject`
  (if (not (`self.IsLocked`))
    (`parent.ReceiveInteractWithObject`)))

(fn `LockDoor`
  (set `self.IsLocked` true))

(fn `UnlockDoor`
  (set `self.IsLocked` false))

(fn `UserConstructionScript`
  (`parent.UserConstructionScript`))