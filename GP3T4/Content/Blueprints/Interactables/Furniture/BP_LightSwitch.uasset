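; BP_LightSwitch is an interactable switch that toggles a referenced set of light actors on and off.
; It applies its IsOn state at BeginPlay, and interaction plays an FMOD switch sound, flipping the state on that node's Finish.
; SetLights stores the state and sets root component visibility on each valid actor in Lights, propagating to children.
; When RemoveBoxes is set, interaction also destroys all actors tagged "Boxes".
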(event `self.ReceiveBeginPlay`
  (`self.SetLights` (`self.IsOn`)))

(event `self.ReceiveInteractWithObject`
  (`/Game/Blueprints/Macros/BP_FMODMacros.PlayFMODEvent` "/Game/FMOD/Events/Lightswitch.Lightswitch" (`self.GetTransform`)
    (:`Finish`
      (`self.SetLights` (not (`self.IsOn`)))
      (if (`self.RemoveBoxes`)
        (bind _outactors (`GameplayStatics.GetAllActorsWithTag` "Boxes"))
        (`self.K2_DestroyActor` _outactors)))))

(fn `SetLights`
  (params (TurnOn :type Boolean))
  (bind _output_get (set `self.IsOn` TurnOn))
  (for _array_element (`self.Lights`)
    (`/Engine/EditorBlueprintResources/StandardMacros.IsValid` _array_element
      (:`Is Valid`
        (`SceneComponent.SetVisibility` (`Actor.RootComponent` _array_element) _output_get true)))))

(fn `UserConstructionScript`)