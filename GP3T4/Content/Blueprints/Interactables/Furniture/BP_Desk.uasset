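; Interactable desk that toggles its four drawers open and closed when the player interacts with it.
; Interaction is ignored mid-animation; otherwise it plays an FMOD door sound, whose Finish output starts the Open or Close timeline.
; Both timelines feed a lerped Y offset into AnimateDrawers, which clamps three drawers to progressively shorter travel, creating a staggered, stepped open pose.
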(event `self.ReceiveBeginPlay`
  (bind _y (.y (`SceneComponent.RelativeLocation` (`self.SM_desk__drawer`))))
  ;[0.8106 0.5614 1] Values to animate with
  (set `self.StartY` _y)
  (set `self.EndY` (+ _y 40.0)))

(event `self.ReceiveInteractWithObject`
  (bind _returnvalue (`self.GetTransform`))
  (if (`self.IsAnimating`)
    _
    (elif (`self.IsOpen`)
      (`/Game/Blueprints/Macros/BP_FMODMacros.PlayFMODEvent` "/Game/FMOD/Events/Dooropen.Dooropen" _returnvalue
        (:`Finish`
          (`self.Close`)))
      (else
        (`/Game/Blueprints/Macros/BP_FMODMacros.PlayFMODEvent` "/Game/FMOD/Events/Dooropen.Dooropen" _returnvalue
          (:`Finish`
            (`self.Open`)))))))

(event `Open`
  ;[0.4533 1 0.4621] Open
  (set `self.IsAnimating` true)
  (bind (_direction _alpha) (`Timeline|OpenTimeLine` :!via `PlayFromStart`)
    (:`Update`
      (`self.AnimateDrawers` (`KismetMathLibrary.Lerp` (`self.StartY`) (`self.EndY`) _alpha)))
    (:`Finished`
      (set `self.IsAnimating` false)
      (set `self.IsOpen` true))))

(event `Close`
  ;[1 0.4405 0.3708] Close
  (set `self.IsAnimating` true)
  (bind (_direction _alpha) (`Timeline|Timeline_0` :!via `PlayFromStart`)
    (:`Update`
      (`self.AnimateDrawers` (`KismetMathLibrary.Lerp` (`self.EndY`) (`self.StartY`) _alpha)))
    (:`Finished`
      (set `self.IsAnimating` false)
      (set `self.IsOpen` false))))

(fn `AnimateDrawers`
  (params (DistanceForward :type "Float (double-precision)"))
  (bind _sm_desk__drawer (`self.SM_desk__drawer`))
  (bind _sm_desk__drawer1 (`self.SM_desk__drawer1`))
  (bind _sm_desk__drawer2 (`self.SM_desk__drawer2`))
  (bind _sm_desk__drawer3 (`self.SM_desk__drawer3`))
  (`SceneComponent.K2_SetRelativeLocation` _sm_desk__drawer (`KismetMathLibrary.MakeVector` (.x (`SceneComponent.RelativeLocation` _sm_desk__drawer)) DistanceForward (.z (`SceneComponent.RelativeLocation` _sm_desk__drawer))) false false)
  (`SceneComponent.K2_SetRelativeLocation` _sm_desk__drawer1 (`KismetMathLibrary.MakeVector` (.x (`SceneComponent.RelativeLocation` _sm_desk__drawer1)) (`KismetMathLibrary.FClamp` DistanceForward (`self.StartY`) (- (`self.EndY`) 10.0)) (.z (`SceneComponent.RelativeLocation` _sm_desk__drawer1))) false false)
  (`SceneComponent.K2_SetRelativeLocation` _sm_desk__drawer2 (`KismetMathLibrary.MakeVector` (.x (`SceneComponent.RelativeLocation` _sm_desk__drawer2)) (`KismetMathLibrary.FClamp` DistanceForward (`self.StartY`) (- (`self.EndY`) 20.0)) (.z (`SceneComponent.RelativeLocation` _sm_desk__drawer2))) false false)
  (`SceneComponent.K2_SetRelativeLocation` _sm_desk__drawer3 (`KismetMathLibrary.MakeVector` (.x (`SceneComponent.RelativeLocation` _sm_desk__drawer3)) (`KismetMathLibrary.FClamp` DistanceForward (`self.StartY`) (- (`self.EndY`) 30.0)) (.z (`SceneComponent.RelativeLocation` _sm_desk__drawer3))) false false))

(fn `UserConstructionScript`)