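; BP_Door is an interactable hinged door that swings between its placed rotation and 90 degrees of yaw from it.
; Interacting, ignored mid-swing, plays the same FMOD door sound for either direction, then calls Open or Close when it finishes.
; Separate timelines lerp the Doorhinge's world rotation and update the state flags.
; OpenDoor and CloseDoor functions trigger the swings directly, without sound or guard.
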(event `self.ReceiveBeginPlay`
  (bind _returnvalue (`self.K2_GetActorRotation`))
  (set `self.ClosedRotation` _returnvalue)
  (set `self.OpenRotation` (`KismetMathLibrary.MakeRotator` (.roll _returnvalue) (.pitch _returnvalue) (+ (.yaw _returnvalue) 90.0))))

(event `self.ReceiveInteractWithObject`
  (bind _returnvalue (`self.GetTransform`))
  (if (`self.IsAnimPlaying`)
    _
    (elif (`self.IsOpen`)
      (`/Game/Blueprints/Macros/BP_FMODMacros.PlayFMODEvent` "/Game/FMOD/Events/Dooropen.Dooropen" _returnvalue
        (:`Finish`
          (`self.Close`)))
      (else
        (`/Game/Blueprints/Macros/BP_FMODMacros.PlayFMODEvent` "/Game/FMOD/Events/Dooropen.Dooropen" _returnvalue
          (:`Finish`
            (`self.Open`)))))))

(event `Open`
  (set `self.IsAnimPlaying` true)
  (bind (_direction _opentrack) (`Timeline|OpenTimeLine` :!via `PlayFromStart`)
    (:`Update`
      (`SceneComponent.K2_SetWorldRotation` (`self.Doorhinge`) (`KismetMathLibrary.RLerp` (`self.ClosedRotation`) (`self.OpenRotation`) _opentrack) false false))
    (:`Finished`
      (set `self.IsAnimPlaying` false)
      (set `self.IsOpen` true))))

(event `Close`
  (set `self.IsAnimPlaying` true)
  (bind (_direction _closetrack) (`Timeline|CloseTimeLine` :!via `PlayFromStart`)
    (:`Update`
      (`SceneComponent.K2_SetWorldRotation` (`self.Doorhinge`) (`KismetMathLibrary.RLerp` (`self.ClosedRotation`) (`self.OpenRotation`) _closetrack) false false))
    (:`Finished`
      (set `self.IsAnimPlaying` false)
      (set `self.IsOpen` false))))

(fn `CloseDoor`
  (`self.Close`))

(fn `OpenDoor`
  (`self.Open`))

(fn `UserConstructionScript`)