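; BP_Meteorite is a meteorite interactable that can flock, be picked up and be shot, handling its sound and destruction effect.
; Tick switches on CurrentState, starting an FMOD comet sound when shooting, then updating its transform, and resetting the play flag in other states.
; On destroy it spawns BP_SmallExplosion, scaling particle size, radius and speeds up sharply when LifeSpanShooting reaches a threshold.
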(event `self.ReceiveTick`
  (params (DeltaSeconds :type "Float (single-precision)"))
  (switch `EMeteoriteState` (`self.CurrentState`)
    (:`FlockingState`
      (set `self.HasPlayed` false :!label _label))
    (:`PickedUpState`
      (goto _label))
    (:`ShootingState`
      (if (`self.HasPlayed`)
        (`FMODBlueprintStatics.EventInstanceSetTransform` (`self.Instance`) (`self.GetTransform`))
        (else
          (bind _instance (`/Game/Blueprints/Macros/BP_FMODMacros.PlayFMODEvent` "/Game/FMOD/Events/Cometshoot.Cometshoot" (`self.GetTransform`))
            (:`Finish`
              (set `self.Instance` _instance)
              (set `self.HasPlayed` true))))))))

(event `self.ReciveOnDestroy`
  (bind _returnvalue (+ (* (`KismetMathLibrary.Conv_BoolToDouble` (>= (`self.LifeSpanShooting`) 0.5)) 35.0) 1.0))
  (bind _returnvalue_2 (`|SpawnActorFromClass` "/Game/VFX/BP_SmallExplosion.BP_SmallExplosion_C" (`self.GetTransform`) "Undefined" "OverrideRootScale" null null))
  (bind _explosioneffect (`/Game/VFX/BP_SmallExplosion.ExplosionEffect` _returnvalue_2))
  (`FXSystemComponent.SetFloatParameter` _explosioneffect "Scale Factor" (* 0.5 _returnvalue))
  (`FXSystemComponent.SetFloatParameter` _explosioneffect "Spawn Radius" (* 20.0 _returnvalue))
  (`FXSystemComponent.SetFloatParameter` _explosioneffect "Min Speed" (* 200.0 _returnvalue))
  (`FXSystemComponent.SetFloatParameter` _explosioneffect "Max Speed" (* 750.0 _returnvalue))
  (`ActorComponent.Activate` _explosioneffect false))

(fn `UserConstructionScript`)