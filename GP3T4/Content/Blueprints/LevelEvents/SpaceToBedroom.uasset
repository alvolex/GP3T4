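; Level-event actor that moves the player from the space sublevel back to the bedroom through a fall-asleep and wake-up transition.
; FallAsleep uses timelines to lower a camera post-process focal value and fade in a black-screen widget, then streams out space and streams in both bedroom sublevels.
; After a short delay, WakeUp fades the black out and raises the focal value.
; A separate HideBedroom event unloads the bedroom sublevels.
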(event `HideBedroom`
  (`self.UnloadBedroomWalls`)
  (`self.UnloadBedroomFloorFurniture`))

(event `self.ReceiveBeginPlay`)

(event `FallAsleep`
  (bind _returnvalue (`GameplayStatics.GetActorOfClass` "/Game/FirstPerson/Blueprints/BP_FirstPersonCharacter.BP_FirstPersonCharacter_C"))
  (bind (_direction _focaldown) (`Timeline|FocalLower` :!via `PlayFromStart`)
    (:`Update`
      (set `CameraComponent.PostProcessSettings` (make `PostProcessSettings` :`DepthOfFieldFocalDistance` _focaldown) (`self.GetComponentByClass` _returnvalue "/Script/Engine.CameraComponent"))
      (`/Engine/EditorBlueprintResources/StandardMacros.DoOnce` false
        (:`Completed`
          (bind _returnvalue_2 (`|CreateWidget` "/Game/My_Widgets/Widget_BlackScreen.Widget_BlackScreen_C"))
          (`UserWidget.AddToViewport` _returnvalue_2 0)
          (if (<= _focaldown 1.0)
            (`TimelineComponent.Stop` (`self.FocalLower`))
            (bind (_direction_2 _brightnessdown) (`Timeline|BrightnessLower` :!label _label)
              (:`Update`
                (`Image.SetColorAndOpacity` (`/Game/My_Widgets/Widget_BlackScreen.BlackScreen` _returnvalue_2) (make `LinearColor` 0.0 0.0 0.0 _brightnessdown))
                (if (>= _brightnessdown 1.0)
                  (`TimelineComponent.Stop` (`self.BrightnessLower`))
                  ;[1 1 1] UNLOAD SPACE
                  (`self.UnloadSpace`)
                  ;[1 1 1] RELOAD BEDROOM
                  (`self.LoadBedroomWallsCeiling`)
                  (`self.LoadBedroomFloorFurniture`)
                  (`KismetSystemLibrary.Delay` 2.0)
                  (`self.WakeUp`))))
            (else
              (goto _label :!via `PlayFromStart`))))))))

(event `WakeUp`
  (bind (_direction _newtrack_0) (`Timeline|BrightnessUp` :!via `PlayFromStart`)
    (:`Update`
      (`Image.SetColorAndOpacity` (`/Game/My_Widgets/Widget_BlackScreen.BlackScreen` (stale `FallAsleep` _returnvalue_2)) (make `LinearColor` 0.0 0.0 0.0 _newtrack_0))
      (if (<= _newtrack_0 0.0)
        (`TimelineComponent.Stop` (`self.BrightnessUp`))
        (bind (_direction_2 _newtrack_0_2) (`Timeline|Focal Up` :!label _label_2)
          (:`Update`
            (bind _returnvalue (`GameplayStatics.GetActorOfClass` "/Game/FirstPerson/Blueprints/BP_FirstPersonCharacter.BP_FirstPersonCharacter_C"))
            (set `CameraComponent.PostProcessSettings` (make `PostProcessSettings` :`DepthOfFieldFocalDistance` _newtrack_0_2) (`self.GetComponentByClass` _returnvalue "/Script/Engine.CameraComponent"))
            (if (>= _newtrack_0_2 500.0)
              (`TimelineComponent.Stop` (`self.Focal Up`)))))
        (else
          (goto _label_2 :!via `PlayFromStart`))))))

(event `LoadBedroomWallsCeiling`
  (`GameplayStatics.LoadStreamLevelBySoftObjectPtr` "/Game/Levels/SubTest/BedroomWallsCeiling.BedroomWallsCeiling" true))

(event `LoadBedroomFloorFurniture`
  (`GameplayStatics.LoadStreamLevelBySoftObjectPtr` "/Game/Levels/SubTest/BedroomFloorFurniture.BedroomFloorFurniture" true))

(event `UnloadBedroomWalls`
  (`GameplayStatics.UnloadStreamLevelBySoftObjectPtr` "/Game/Levels/SubTest/BedroomWallsCeiling.BedroomWallsCeiling"))

(event `UnloadBedroomFloorFurniture`
  (`GameplayStatics.UnloadStreamLevelBySoftObjectPtr` "/Game/Levels/SubTest/BedroomFloorFurniture.BedroomFloorFurniture"))

(event `UnloadSpace`
  (`GameplayStatics.UnloadStreamLevelBySoftObjectPtr` "/Game/Levels/SubTest/SpaceSubLevel.SpaceSubLevel"))

(fn `UserConstructionScript`)