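; Legacy level-event Blueprint for sleep and wake transitions between the bedroom and space levels; its events are empty and its logic is disconnected.
; The leftover graph streams bedroom, space, corridor and door sublevels, chosen by ShouldLoadSpace and ShouldLoadBedroom flags.
; It also holds camera focal and black-screen fade timelines, HUD fades, player repositioning and look-rotation locking.
; A note on FallAsleep says it moved to BP_LevelTransitionMacros.
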(event `FallAsleep`
  ;[0 0 0] Moved to BP_LevelTransitionMacros
)

(event `self.ReceiveTick`
  (params (DeltaSeconds :type "Float (single-precision)"))
  ;[0 0 0] Moved to BP_LevelTransitionMacros
)

(event `HideBedroom`
  ;[0 0 0] Moved to BP_LevelTransitionMacros
)

(event `LoadBedroomWallsCeiling`
  ;[0 0 0] Moved to BP_LevelTransitionMacros
)

(event `LoadBedroomFloorFurniture`
  ;[0 0 0] Moved to BP_LevelTransitionMacros
)

(event `BackToBedroom`
  ;[0 0 0] Moved to BP_LevelTransitionMacros
  ;;[0 1 0.5529] When Level Done - BACK TO BEDROOM
)

(event `UnloadBedroomWalls`
  ;[0 0 0] Moved to BP_LevelTransitionMacros
)

(event `UnloadBedroomFloorFurniture`
  ;[0 0 0] Moved to BP_LevelTransitionMacros
)

(event `UnloadBedroom`
  ;[0 0 0] Moved to BP_LevelTransitionMacros
)

(event `LoadBedroom`
  ;[0 0 0] Moved to BP_LevelTransitionMacros
)

(event `LoadSpace`
  ;[0 0 0] Moved to BP_LevelTransitionMacros
)

(event `WakeUp`
  ;[0 0 0] Moved to BP_LevelTransitionMacros
)

(event `UnloadSpace`
  ;[0 0 0] Moved to BP_LevelTransitionMacros
)

(event `LoadCorridor`
  ;[0 0 0] Moved to BP_LevelTransitionMacros
)

(event `UnloadCorridor`
  ;[0 0 0] Moved to BP_LevelTransitionMacros
)

(fn `UserConstructionScript`)