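; City level trigger that collapses a referenced building the first time an actor overlaps it.
; On overlap, a DoOnce enables physics simulation on the building's facade, back, left and right wall components.
; After a short delay it switches their physics back off and prints a debug message.
; A player-character check exists but is disconnected, so any overlapping actor can fire the trigger.
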(event `self.ReceiveActorBeginOverlap`
  (params (OtherActor :type "Actor Object Reference"))
  (`/Engine/EditorBlueprintResources/StandardMacros.DoOnce` false
    (:`Completed`
      (`PrimitiveComponent.SetSimulatePhysics` (`/Game/Blueprints/LevelEvents/Level_City/BP_City_Building_Shatter_1.Facade1` (`self.Ref_Building`)) true)
      (`PrimitiveComponent.SetSimulatePhysics` (`/Game/Blueprints/LevelEvents/Level_City/BP_City_Building_Shatter_1.Wall_Back` (`self.Ref_Building`)) true)
      (`PrimitiveComponent.SetSimulatePhysics` (`/Game/Blueprints/LevelEvents/Level_City/BP_City_Building_Shatter_1.Wall_Left` (`self.Ref_Building`)) true)
      (`PrimitiveComponent.SetSimulatePhysics` (`/Game/Blueprints/LevelEvents/Level_City/BP_City_Building_Shatter_1.Wall_Right` (`self.Ref_Building`)) true)
      (`KismetSystemLibrary.Delay` 5.0)
      (`PrimitiveComponent.SetSimulatePhysics` (`/Game/Blueprints/LevelEvents/Level_City/BP_City_Building_Shatter_1.Facade1` (`self.Ref_Building`)) false)
      (`PrimitiveComponent.SetSimulatePhysics` (`/Game/Blueprints/LevelEvents/Level_City/BP_City_Building_Shatter_1.Wall_Back` (`self.Ref_Building`)) false)
      (`PrimitiveComponent.SetSimulatePhysics` (`/Game/Blueprints/LevelEvents/Level_City/BP_City_Building_Shatter_1.Wall_Left` (`self.Ref_Building`)) false)
      (`PrimitiveComponent.SetSimulatePhysics` (`/Game/Blueprints/LevelEvents/Level_City/BP_City_Building_Shatter_1.Wall_Right` (`self.Ref_Building`)) false)
      (`KismetSystemLibrary.PrintString` "Stop physics"))))

(fn `UserConstructionScript`)