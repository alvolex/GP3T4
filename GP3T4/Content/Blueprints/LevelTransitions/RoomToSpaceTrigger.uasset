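; Level-transition trigger that swaps the bedroom out for what appears to be a space scene, then wakes the player back in bed.
; Player overlap with any of four box colliders, identified by the IsPlayerCharacter interface, hides the bedroom and starts a timer.
; When the timer finishes, chained steps fade to black, restore the bedroom, run SpaceToCorridor, then teleport and orient the player to BP_Bed's wake-up point as it fades in.
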(event `self.TimerFinished`
  (`/Game/Blueprints/Macros/BP_LevelTransitionMacros.FadeToBlack` 2.0
    (:`End`
      (`KismetSystemLibrary.Delay` 2.0)
      (`/Game/Blueprints/Macros/BP_LevelTransitionMacros.ShowBedroom`
        (:`End`
          (`/Game/Blueprints/Macros/BP_LevelTransitionMacros.SpaceToCorridor`
            (:`End`
              (bind _returnvalue (`GameplayStatics.GetActorOfClass` "/Game/Blueprints/Interactables/Furniture/BP_Bed.BP_Bed_C"))
              (`/Game/Blueprints/Interactables/Furniture/BP_Bed.FadeToNormal` _returnvalue 2.0)
              (bind _wakeupposition (`/Game/Blueprints/Interactables/Furniture/BP_Bed.WakeUpPosition` _returnvalue))
              (`self.K2_SetActorLocation` (`GameplayStatics.GetPlayerCharacter` 0) (`SceneComponent.K2_GetComponentLocation` _wakeupposition) false true)
              (`Controller.SetControlRotation` (`GameplayStatics.GetPlayerController` 0) (`SceneComponent.K2_GetComponentRotation` _wakeupposition)))))))))

(event `self.BoxCollider_0.OnComponentBeginOverlap`
  (params (OverlappedComponent :type "PrimitiveComponent Object Reference") (OtherActor :type "Actor Object Reference") (OtherComp :type "PrimitiveComponent Object Reference") (OtherBodyIndex :type Integer) (bFromSweep :type Boolean) (SweepResult :type "HitResult Structure (by ref)"))
  (if (`KismetSystemLibrary.DoesImplementInterface` OtherActor "/Script/GP3T4.IsPlayerCharacter")
    (`/Game/Blueprints/Macros/BP_LevelTransitionMacros.HideBedroom` :!label _label
      (:`End`
        (`self.StartTimer`)))))

(event `self.BoxCollider_1.OnComponentBeginOverlap`
  (params (OverlappedComponent :type "PrimitiveComponent Object Reference") (OtherActor :type "Actor Object Reference") (OtherComp :type "PrimitiveComponent Object Reference") (OtherBodyIndex :type Integer) (bFromSweep :type Boolean) (SweepResult :type "HitResult Structure (by ref)"))
  (if (`KismetSystemLibrary.DoesImplementInterface` OtherActor "/Script/GP3T4.IsPlayerCharacter")
    (goto _label)))

(event `self.BoxCollider_2.OnComponentBeginOverlap`
  (params (OverlappedComponent :type "PrimitiveComponent Object Reference") (OtherActor :type "Actor Object Reference") (OtherComp :type "PrimitiveComponent Object Reference") (OtherBodyIndex :type Integer) (bFromSweep :type Boolean) (SweepResult :type "HitResult Structure (by ref)"))
  (if (`KismetSystemLibrary.DoesImplementInterface` OtherActor "/Script/GP3T4.IsPlayerCharacter")
    (goto _label)))

(event `self.BoxCollider_3.OnComponentBeginOverlap`
  (params (OverlappedComponent :type "PrimitiveComponent Object Reference") (OtherActor :type "Actor Object Reference") (OtherComp :type "PrimitiveComponent Object Reference") (OtherBodyIndex :type Integer) (bFromSweep :type Boolean) (SweepResult :type "HitResult Structure (by ref)"))
  (if (`KismetSystemLibrary.DoesImplementInterface` OtherActor "/Script/GP3T4.IsPlayerCharacter")
    (goto _label)))

(fn `UserConstructionScript`)