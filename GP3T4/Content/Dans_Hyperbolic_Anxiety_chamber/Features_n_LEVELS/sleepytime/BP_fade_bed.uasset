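; Interactable bed that fades the screen to black and back once, for the sleep sequence.
; Interaction plays the HUD fade widget forward and binds to its animation end; after a hold delay, the animation plays in reverse.
; A separate InterpPP event, not triggered by the interaction, blends in a sleeping post-process on the camera, restores normal settings, then calls FallAsleep on BedroomToSpace.
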(event `self.ReceiveInteractWithObject`
  (`/Engine/EditorBlueprintResources/StandardMacros.DoOnce` false
    (:`Completed`
      (`self.FadeToBlack` (`self.Fade_IN_Duration`)))))

(event `FinishedFading`
  (`KismetSystemLibrary.Delay` (`self.Fade_HOLD_Duration`))
  (`self.FadeToNormal` (`self.Fade_OUT_Duration`)))

(event `InterpPP`
  (if (`self.bInterpPP`)
    (if (`KismetSystemLibrary.IsValid` (`self.First Person Camera Component`))
      (set `CameraComponent.PostProcessSettings` (`self.SleepingPostProcess`) (`self.First Person Camera Component`))
      (bind (_direction _ppvalue) (`Timeline|Interp` :`NewTime` 5.0 :!via `PlayFromStart`)
        (:`Update`
          (if (`KismetSystemLibrary.IsValid` (`self.First Person Camera Component`))
            (`CameraComponent.SetPostProcessBlendWeight` (`self.First Person Camera Component`) _ppvalue)
            (`KismetSystemLibrary.PrintString` "INTERPOLATING" true true (struct :`G` 0.66 :`B` 1.0 :`A` 1.0) 0.0)))
        (:`Finished`
          (set `CameraComponent.PostProcessSettings` (`self.NormalPostProcess`) (`self.First Person Camera Component`))
          (bind _returnvalue (`GameplayStatics.GetActorOfClass` "/Game/Blueprints/LevelEvents/BedroomToSpace.BedroomToSpace_C"))
          (`/Game/Blueprints/LevelEvents/BedroomToSpace.FallAsleep` _returnvalue))))))

(fn `FadeToBlack`
  (params (PlaybackSpeed :type "Float (single-precision)"))
  (bind _asbp_player_hud (cast `/Game/Blueprints/HUD/BP_PlayerHUD` (`PlayerController.GetHUD` (`GameplayStatics.GetPlayerController` 0))))
  (bind _fadewidget (`/Game/Blueprints/HUD/BP_PlayerHUD.FadeWidget` _asbp_player_hud))
  (`/Game/Dans_Hyperbolic_Anxiety_chamber/Fade.FadeToBlack` _fadewidget PlaybackSpeed "Forward")
  (`UserWidget.BindToAnimationFinished` _fadewidget (`/Game/Dans_Hyperbolic_Anxiety_chamber/Fade.FadeInBlackScreen` _fadewidget) (`|CreateDelegate` :!event `FinishedFading`)))

(fn `FadeToNormal`
  (params (PlaybackSpeed :type "Float (single-precision)"))
  (bind _asbp_player_hud (cast `/Game/Blueprints/HUD/BP_PlayerHUD` (`PlayerController.GetHUD` (`GameplayStatics.GetPlayerController` 0))))
  (bind _fadewidget (`/Game/Blueprints/HUD/BP_PlayerHUD.FadeWidget` _asbp_player_hud))
  (`UserWidget.UnbindFromAnimationFinished` _fadewidget (`/Game/Dans_Hyperbolic_Anxiety_chamber/Fade.FadeInBlackScreen` _fadewidget) (`|CreateDelegate` :!event `FinishedFading`))
  (`/Game/Dans_Hyperbolic_Anxiety_chamber/Fade.FadeToBlack` _fadewidget PlaybackSpeed "Reverse"))

(fn `StartFade`
  (params (PlaybackSpeed :type "Float (single-precision)") (PlayMode :type "EUMGSequencePlayMode Enum" :default "Forward"))
  (bind _asbp_player_hud (cast `/Game/Blueprints/HUD/BP_PlayerHUD` (`PlayerController.GetHUD` (`GameplayStatics.GetPlayerController` 0))))
  (`/Game/Dans_Hyperbolic_Anxiety_chamber/Fade.FadeToBlack` (`/Game/Blueprints/HUD/BP_PlayerHUD.FadeWidget` _asbp_player_hud) PlaybackSpeed PlayMode))

(fn `UserConstructionScript`)