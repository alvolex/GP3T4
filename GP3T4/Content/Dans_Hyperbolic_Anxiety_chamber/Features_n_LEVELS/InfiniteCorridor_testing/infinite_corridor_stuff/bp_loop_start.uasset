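; Corridor segment actor for an infinite looping hallway, spawning the next segment as the player walks through.
; On the player's first box overlap it locks and closes its child-actor door and destroys the previous corridor.
; It then spawns another Bp_loop_start at a placement component, passing itself and an incremented loop count.
; When the count equals LoopUntilSwitch, it spawns a Bp_loop_end with the count reset instead.
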(event `self.ReceiveBeginPlay`
  (bind _asbp_lockable_door (cast `/Game/Blueprints/Interactables/BP_Lockable_Door` (`ChildActorComponent.ChildActor` (`self.BP_Lockable_Door`))))
  (set `self.lockable_door` _asbp_lockable_door)
  (`KismetSystemLibrary.PrintText` (`KismetTextLibrary.Conv_IntToText` (`self.Loop_Number`))))

(event `self.Box.OnComponentBeginOverlap`
  (params (OverlappedComponent :type "PrimitiveComponent Object Reference") (OtherActor :type "Actor Object Reference") (OtherComp :type "PrimitiveComponent Object Reference") (OtherBodyIndex :type Integer) (bFromSweep :type Boolean) (SweepResult :type "HitResult Structure (by ref)"))
  (bind _lockable_door (`self.lockable_door`))
  (bind _previouscorridor (`self.PreviousCorridor`))
  (bind _returnvalue (`SceneComponent.K2_GetComponentToWorld` (`self.NewCorridorPlacement`)))
  (if (and (== OtherActor (`Controller.K2_GetPawn` (`GameplayStatics.GetPlayerController` 0))) (not (`self.HasBeenThrough`)))
    (set `self.HasBeenThrough` true)
    (`/Game/Blueprints/Interactables/BP_Lockable_Door.LockDoor` _lockable_door)
    (`/Game/Blueprints/Interactables/BP_Door.CloseDoor` _lockable_door)
    (`|ExecutionSequence`
      (:`then_0`
        (`/Engine/EditorBlueprintResources/StandardMacros.IsValid` _previouscorridor
          (:`Is Valid`
            (`self.K2_DestroyActor` _previouscorridor))))
      (:`then_1`
        (if (== (`self.Loop_Number`) (`self.Loop_Until_Switch`))
          (bind _returnvalue_2 (`|SpawnActorFromClass` "/Game/Dans_Hyperbolic_Anxiety_chamber/Features_n_LEVELS/InfiniteCorridor_testing/infinite_corridor_stuff/bp_loop_end.bp_loop_end_C" _returnvalue "Undefined" "OverrideRootScale" null null))
          (set `self.PreviousCorridor` self)
          (set `/Game/Dans_Hyperbolic_Anxiety_chamber/Features_n_LEVELS/InfiniteCorridor_testing/infinite_corridor_stuff/bp_loop_end.Loop_Number` 0 _returnvalue_2)
          (`KismetSystemLibrary.PrintText` "NEW LOOP STARTED")
          (else
            (bind _returnvalue_3 (`|SpawnActorFromClass` "bp_loop_start_C" _returnvalue "AlwaysSpawn" "OverrideRootScale" null null))
            (set `/Game/Dans_Hyperbolic_Anxiety_chamber/Features_n_LEVELS/InfiniteCorridor_testing/infinite_corridor_stuff/bp_loop_start.PreviousCorridor` self _returnvalue_3)
            (bind _result (`/Engine/EditorBlueprintResources/StandardMacros.IncrementInt` (`self.Loop_Number`))
              (:`  `
                (bind _output_get (set `/Game/Dans_Hyperbolic_Anxiety_chamber/Features_n_LEVELS/InfiniteCorridor_testing/infinite_corridor_stuff/bp_loop_start.Loop_Number` _result _returnvalue_3))
                (`KismetSystemLibrary.PrintText` (`KismetTextLibrary.Conv_IntToText` _output_get))))))))))

(fn `UserConstructionScript`)