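; Infinite-corridor segment that chains copies of itself to form a looping hallway, ending in a switch to the city level.
; When the player first enters its trigger box, it locks and closes its child-actor door, then runs a destroy pass over the tracked previous corridors.
; At the final loop count it opens City_Leveldesign_Axel; otherwise it spawns right and left successors, passing on an incremented LoopNumber and recording corridors in PreviousCorridor.
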(event `self.ReceiveBeginPlay`
  (bind _asbp_lockable_door (cast `/Game/Blueprints/Interactables/BP_Lockable_Door` (`ChildActorComponent.ChildActor` (`self.BP_Lockable_Door`))))
  (set `self.lockable_door` _asbp_lockable_door)
  (`KismetSystemLibrary.PrintText` (`KismetTextLibrary.Conv_IntToText` (`self.Loop_Number`))))

(event `self.Box.OnComponentBeginOverlap`
  (params (OverlappedComponent :type "PrimitiveComponent Object Reference") (OtherActor :type "Actor Object Reference") (OtherComp :type "PrimitiveComponent Object Reference") (OtherBodyIndex :type Integer) (bFromSweep :type Boolean) (SweepResult :type "HitResult Structure (by ref)"))
  (bind _lockable_door (`self.lockable_door`))
  (if (and (== OtherActor (`Controller.K2_GetPawn` (`GameplayStatics.GetPlayerController` 0))) (not (`self.HasBeenThrough`)))
    (set `self.HasBeenThrough` true)
    (`/Game/Blueprints/Interactables/BP_Lockable_Door.LockDoor` _lockable_door)
    (`/Game/Blueprints/Interactables/BP_Door.CloseDoor` _lockable_door)
    (`KismetArrayLibrary.Array_RemoveItem` (`self.PreviousCorridor`) self)
    (`|ExecutionSequence`
      (:`then_0`
        (for _array_element (`self.PreviousCorridor`)
          (`/Engine/EditorBlueprintResources/StandardMacros.IsValid` _array_element
            (:`Is Valid`
              (`self.K2_DestroyActor`)))))
      (:`then_1`
        (if (== (`self.Loop_Number`) 4)
          (`GameplayStatics.OpenLevelBySoftObjectPtr` "/Game/Levels/City_Leveldesign_Axel.City_Leveldesign_Axel")
          (else
            (`|ExecutionSequence`
              (:`then_0`
                (bind _returnvalue (`|SpawnActorFromClass` "bp_loop_end_C" (`SceneComponent.K2_GetComponentToWorld` (`self.RightCorridor`)) "Undefined" "OverrideRootScale" null null))
                (`KismetArrayLibrary.Array_Set` (`self.PreviousCorridor`) 0 _returnvalue)
                (bind _result (`/Engine/EditorBlueprintResources/StandardMacros.IncrementInt` (`self.Loop_Number`))
                  (:`  `
                    (bind _output_get (set `/Game/Dans_Hyperbolic_Anxiety_chamber/Features_n_LEVELS/InfiniteCorridor_testing/infinite_corridor_stuff/bp_loop_end.Loop_Number` _result _returnvalue))
                    (`KismetSystemLibrary.PrintText` (`KismetTextLibrary.Conv_IntToText` _output_get)))))
              (:`then_1`
                (bind _returnvalue_2 (`|SpawnActorFromClass` "bp_loop_end_C" (`SceneComponent.K2_GetComponentToWorld` (`self.LeftCorridor`)) "Undefined" "OverrideRootScale" null null))
                (`KismetArrayLibrary.Array_Set` (`self.PreviousCorridor`) 1)
                (bind _result_2 (`/Engine/EditorBlueprintResources/StandardMacros.IncrementInt` (`self.Loop_Number`))
                  (:`  `
                    (set `/Game/Dans_Hyperbolic_Anxiety_chamber/Features_n_LEVELS/InfiniteCorridor_testing/infinite_corridor_stuff/bp_loop_end.Loop_Number` _result_2 _returnvalue_2)
                    (`KismetArrayLibrary.Array_Set` (`self.PreviousCorridor`) 2 self)))))))))))

(fn `UserConstructionScript`)