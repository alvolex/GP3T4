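; Eye component that keeps itself turned toward player character 0, aiming slightly above the actor's location.
; Every Tick it builds a look-at basis from the direction to that point using cross products with world up.
; It applies the result as world rotation with pitch and roll swapped and yaw offset a quarter turn.
; An angle check against the attach parent's right vector is left unconnected, so rotation has no limit.
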(event `self.ReceiveTick`
  (params (DeltaSeconds :type "Float (single-precision)"))
  (bind _returnvalue (- (+ (`Actor.K2_GetActorLocation` (`GameplayStatics.GetPlayerCharacter` 0)) (0.0 0.0 50.0)) (`self.K2_GetComponentLocation`)))
  (bind _returnvalue_2 (`KismetMathLibrary.Cross_VectorVector` _returnvalue (`KismetMathLibrary.Vector_Up`)))
  (bind (_returnvalue_roll _returnvalue_pitch _returnvalue_yaw) (`KismetMathLibrary.BreakRotator` (`KismetMathLibrary.MakeRotationFromAxes` _returnvalue _returnvalue_2 (`KismetMathLibrary.Cross_VectorVector` _returnvalue_2 _returnvalue))))
  (`/Engine/EditorBlueprintResources/StandardMacros.IsValid` (`GameplayStatics.GetPlayerCharacter` 0)
    (:`Is Valid`
      ;[0.5297 1 0.5153] Rotate the eye
      (`self.K2_SetWorldRotation` (`KismetMathLibrary.MakeRotator` _returnvalue_pitch _returnvalue_roll (- _returnvalue_yaw 90.0))))))